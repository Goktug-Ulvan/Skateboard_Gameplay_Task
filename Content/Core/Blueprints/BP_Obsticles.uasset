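; BP_Obsticles is an obstacle that awards points when the player pawn overlaps it during a kickflip.
; The construction script writes its Score onto a text label, which yaws toward the player every Tick.
; On box overlap it queries the pawn's kickflip state by interface, then sends Score to the player state by interface and destroys itself.
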(event `self.ReceiveTick`
  (params (DeltaSeconds :type "Float (single-precision)"))
  (bind (_returnvalue_roll _returnvalue_pitch _returnvalue_yaw) (`KismetMathLibrary.BreakRotator` (`KismetMathLibrary.FindLookAtRotation` (`self.K2_GetActorLocation`) (`self.K2_GetActorLocation` (`GameplayStatics.GetPlayerPawn` 0)))))
  (`SceneComponent.K2_SetWorldRotation` (`self.TextRender`) (`KismetMathLibrary.MakeRotator` 0.0 0.0 _returnvalue_yaw) false false))

(event `self.Box.OnComponentBeginOverlap`
  (params (OverlappedComponent :type "PrimitiveComponent Object Reference") (OtherActor :type "Actor Object Reference") (OtherComp :type "PrimitiveComponent Object Reference") (OtherBodyIndex :type Integer) (bFromSweep :type Boolean) (SweepResult :type "HitResult Structure (by ref)"))
  (bind _returnvalue (`GameplayStatics.GetPlayerPawn` 0))
  (if (== OtherActor _returnvalue)
    (bind _return (message `/Game/Core/Interfaces/BPI_Player.BPI_GetKickflip` _returnvalue))
    (if _return
      (message `/Game/Core/Interfaces/BPI_PlayerState.BPI_SetScore` (`GameplayStatics.GetPlayerState` 0) (`self.Score`))
      (`self.K2_DestroyActor`))))

(fn `UserConstructionScript`
  (`TextRenderComponent.K2_SetText` (`self.TextRender`) (`|FormatText` "{points} Points" (`self.Score`))))