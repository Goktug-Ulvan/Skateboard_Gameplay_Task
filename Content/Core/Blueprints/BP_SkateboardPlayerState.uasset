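; Player state Blueprint for the skateboard game that holds the player's current state enum and score points.
; Interface events set the state or add to the score, then fire the state-changed or points-added dispatcher, and interface getters return both values.
; A state change also sends a set-inputs interface message to the player controller.
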(event `/Game/Core/Interfaces/BPI_PlayerState.BPI_SetState`
  (params (input :type "/Game/Core/Enums/E_PlayerState Enum" :default "NewEnumerator0"))
  (set `self.E_PlayerState` input)
  (`self.PlayerStateChanged`)
  (message `/Game/Core/Interfaces/BPI_PlayerController.BPI_SetInputs` (`self.GetPlayerController`)))

(event `/Game/Core/Interfaces/BPI_PlayerState.BPI_SetScore`
  (params (input :type "Float (double-precision)"))
  (set `self.ScorePoints` (+ (`self.ScorePoints`) input))
  (`self.PointsAdded`))

(fn `BPI_GetScore`
  (returns (return :type "Float (double-precision)"))
  (return (`self.ScorePoints`)))

(fn `BPI_GetState`
  (returns (return :type "/Game/Core/Enums/E_PlayerState Enum"))
  (return (`self.E_PlayerState`)))

(fn `UserConstructionScript`)