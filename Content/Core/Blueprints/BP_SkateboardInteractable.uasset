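; BP_SkateboardInteractable is a placeable skateboard that destroys itself when interacted with.
; Its enum selects the board: the construction script calls the mesh setup and shows the enum name on a text render.
; For non-default values, setup queries the GameInstance through an interface using the enum index minus one.
; It async-loads the soft-referenced mesh, then applies the material, or the material instance if none is set.
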(event `Set_Mesh`
  (bind _returnvalue (`GameplayStatics.GetGameInstance`))
  (bind _staticmesh (`self.StaticMesh`))
  (bind _e_interactable (`self.E_Interactable`))
  (if (`|EnumInequality` _e_interactable "NewEnumerator0")
    (`/Engine/EditorBlueprintResources/StandardMacros.IsValid` _returnvalue
      (:`Is Valid`
        (bind (_name _material _m_instance _mesh) (message `/Game/Core/Interfaces/BPI_GameInstance.BPI_GetSkateboards` _returnvalue (- (`KismetMathLibrary.Conv_ByteToInt` _e_interactable) 1)))
        (bind _object (`|LoadAsset` _mesh)
          (:`then`
            (bind _asstatic_mesh (cast `StaticMesh` _object))
            (`StaticMeshComponent.SetStaticMesh` (`self.StaticMesh`) _asstatic_mesh)
            (if (`KismetSystemLibrary.IsValidSoftObjectReference` _material)
              (bind _object_2 (`|LoadAsset` _material)
                (:`then`
                  (bind _asmaterial (cast `Material` _object_2))
                  (`PrimitiveComponent.SetMaterial` _staticmesh 0 _asmaterial)))
              (else
                (bind _object_3 (`|LoadAsset` _m_instance)
                  (:`then`
                    (bind _asmaterial_instance (cast `MaterialInstance` _object_3))
                    (`PrimitiveComponent.SetMaterial` _staticmesh 0 _asmaterial_instance)))))))))))

(event `/Game/Core/Interfaces/BPI_Interaction.OnInteract`
  (`self.K2_DestroyActor`))

(fn `UserConstructionScript`
  (`self.Set_Mesh`)
  (`TextRenderComponent.K2_SetText` (`self.TextRender`) (`KismetTextLibrary.Conv_StringToText` (`|GetEnumeratorNameAsString` (`self.E_Interactable`)))))